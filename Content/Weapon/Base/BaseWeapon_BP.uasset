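; Base weapon Blueprint owned by a BaseCharactor_BP, handling firing, ammo and reload for a gun attached to the character's mesh.
; Fire aims the muzzle, spawns effects and applies point damage on trace hits, zeroed for actors of the filter class.
; Equipping binds owner dispatchers for reload, aim and weapon switch; aim events are empty here.
; Ammo lives in WeaponData, with infinite-ammo support and dispatchers for widget updates and reload requests.
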(event `self.ReceiveBeginPlay`
  ;[1 1 1] 코멘트
  (`SceneComponent.SetVisibility` (`self.SK_FPGun`) false false)
  (set `self.OwnerPawn` (stale _asbase_charactor_bp))
  (bind _asbase_charactor_bp (cast `/Game/Mannequin/Player3/BaseCharactor_BP` (`self.GetOwner`))))

(event `Fire`
  (params (Direction :type "Vector Structure") (`Random Half Angle` :type "Float (double-precision)") (FilterClass :type "/Game/Mannequin/Player3/Base/BP_BaseCharacter Class Reference"))
  (bind (_weapondata_weaponclass _weapondata_hudimage _weapondata_currentammo _weapondata_currentammoinclip) (break `/Game/Weapon/Base/WeaponData` (`self.WeaponData`)))
  (bind (_weapondata_weaponclass_2 _weapondata_hudimage_2 _weapondata_currentammo_2 _weapondata_currentammoinclip_2) (break `/Game/Weapon/Base/WeaponData` (`self.WeaponData`)))
  (`|ExecutionSequence`
    (:`then_0`
      (set `self.ShootDirection` Direction)
      (set `self.RandomConeHalfAngle` `Random Half Angle`)
      (set `self.Filter Class` FilterClass))
    (:`then_1`
      (if (or (`self.bInfiniteAmmo`) (and (not (`self.bIsReloading`)) (not (`self.Is Empty Ammo`))))
        (`SceneComponent.K2_SetWorldRotation` (`self.Muzzle`) (`KismetMathLibrary.MakeRotFromX` (`self.ShootDirection`)) false false)
        (`|ExecutionSequence`
          (:`then_1`
            (`self.SpawnFireEffects`)
            (`self.OnFire`)
            (if (`self.TraceHit`)
              (`GameplayStatics.ApplyPointDamage` (`self.TraceHitActor`) (`KismetMathLibrary.Conv_BoolToDouble` (!= (`GameplayStatics.GetObjectClass` (`self.TraceHitActor`)) (`self.Filter Class`))) (`self.GetTraceDirection`) (`self.TraceHitResult`) (`Pawn.GetController` (`self.OwnerPawn`)) self)
              (`GameplayStatics.SpawnEmitterAtLocation` (`self.BulletImpact`) (`self.TraceHitLocation`))))
          (:`then_2`
            (`/Engine/EditorBlueprintResources/StandardMacros.DecrementInt` _weapondata_currentammoinclip
              (:`  `
                (`self.OnUpdateWidget` (`self.WeaponData`))
                (if (and (<= _weapondata_currentammoinclip_2 0) (not (`self.Is Empty Ammo`)))
                  (`self.OnNeedReload`))))))))))

(event `Equipped`
  ;[1 1 1] 무기 장착
  (`self.K2_AttachToComponent` (`Character.Mesh` (`self.OwnerPawn`)) "None" "SnapToTarget" "SnapToTarget" "KeepRelative")
  (`self.BindingOwnerEventDispatcher`)
  (`self.OnUpdateWidget` (`self.WeaponData`)))

(event `UnEquipped`
  ;[1 1 1] 장착하지 않음
  (`SceneComponent.SetVisibility` (`self.SK_FPGun`) false false))

(event `BeginAim`)

(event `EndAim`)

(event `BindingOwnerEventDispatcher`
  ;[1 1 1] 이벤트 보내주기
  (add `/Game/Mannequin/Player3/BaseCharactor_BP.OnBeginReload` (`self.OwnerPawn`) (`|CreateDelegate` :!event `BeginReload`))
  (add `/Game/Mannequin/Player3/BaseCharactor_BP.OnEndReloaded` (`self.OwnerPawn`) (`|CreateDelegate` :!event `EndReload`))
  (add `/Game/Mannequin/Player3/BaseCharactor_BP.OnBeginAim` (`self.OwnerPawn`) (`|CreateDelegate` :!event `BeginAim`))
  (add `/Game/Mannequin/Player3/BaseCharactor_BP.OnEndAim` (`self.OwnerPawn`) (`|CreateDelegate` :!event `EndAim`))
  (add `/Game/Mannequin/Player3/BaseCharactor_BP.OnSwitchWeaponFinished` (`self.OwnerPawn`) (`|CreateDelegate` :!event `ShowWeaponMeshs`)))

(event `ShowWeaponMeshs`
  (params (NewWeapon :type "/Game/Weapon/Base/BaseWeapon_BP Object Reference"))
  ;[1 1 1] 무기 모형 보여주기 이벤트
  (if (== NewWeapon self)
    (`SceneComponent.SetVisibility` (`self.SK_FPGun`) true false)))

(event `BeginReload`
  ;[1 1 1] 장전 이벤트 시작
  (if (`self.IsOwnerEquipWeapon`)
    (set `self.bIsReloading` true)))

(event `EndReload`
  (bind (_new_current_ammo _new_ammo_clip) (`self.CalcAmmoAfterReload`))
  (bind _weapondata (`self.WeaponData`))
  ;[1 1 1] 장전 이벤트 끝
  (if (not (`self.bInfiniteAmmo`))
    (if (`self.IsOwnerEquipWeapon`)
      (setmembers `/Game/Weapon/Base/WeaponData` :`StructRef` (`self.WeaponData`) :`WeaponClass` null :`HUDImage` null :`CurrentAmmo` _new_current_ammo :`CurrentAmmoInClip` _new_ammo_clip :`AmmoPerClip` 0)
      (else
        (setmembers `/Game/Weapon/Base/WeaponData` :`StructRef` _weapondata :`WeaponClass` null :`HUDImage` null :`CurrentAmmo` 0 :`CurrentAmmoInClip` (`.AmmoPerClip_14_030733AD4351C2A325140680BD235A86` (break `/Game/Weapon/Base/WeaponData` _weapondata)) :`AmmoPerClip` 0)))
    (`self.OnUpdateWidget` (`self.WeaponData`))
    (set `self.bIsReloading` true)))

(fn `CalcAmmoAfterReload`
  (returns (`New Current Ammo` :type Integer) (`New Ammo Clip` :type Integer))
  (locals (UseAmmo :type Integer))
  (bind (_weaponclass _hudimage _currentammo _currentammoinclip _ammoperclip) (break `/Game/Weapon/Base/WeaponData` (`self.WeaponData`)))
  (bind (_weaponclass_2 _hudimage_2 _currentammo_2 _currentammoinclip_2) (break `/Game/Weapon/Base/WeaponData` (`self.WeaponData`)))
  (bind (_weaponclass_3 _hudimage_3 _currentammo_3) (break `/Game/Weapon/Base/WeaponData` (`self.WeaponData`)))
  (set `local.UseAmmo` (- _ammoperclip _currentammoinclip))
  (return (- _currentammo_3 (`KismetMathLibrary.Min` _currentammo_3 (`local.UseAmmo`))) (+ _currentammoinclip_2 (`KismetMathLibrary.Min` _currentammo_2 (`local.UseAmmo`)))))

(fn `Get Muzzle Direction`
  (returns (Direction :type "Vector Structure"))
  (return (`KismetMathLibrary.GetForwardVector` (`SceneComponent.K2_GetComponentRotation` (`self.Muzzle`)))))

(fn `Get Muzzle Location`
  (returns (NewParam :type "Vector Structure"))
  (return (`SceneComponent.K2_GetComponentLocation` (`self.Muzzle`))))

(fn `GetTraceDirection`
  (returns (ReturnValue :type "Vector Structure"))
  (return (`KismetMathLibrary.Normal` (- (`self.TraceEnd`) (`self.TraceStart`)))))

(fn `Is Empty Ammo`
  (returns (NewParam :type Boolean))
  (locals (EmptyAmmo :type Boolean) (EmptyClip :type Boolean))
  (bind (_weapondata_weaponclass _weapondata_hudimage _weapondata_currentammo) (break `/Game/Weapon/Base/WeaponData` (`self.WeaponData`)))
  (bind (_weapondata_weaponclass_2 _weapondata_hudimage_2 _weapondata_currentammo_2 _weapondata_currentammoinclip) (break `/Game/Weapon/Base/WeaponData` (`self.WeaponData`)))
  (set `local.EmptyAmmo` (<= _weapondata_currentammo 0))
  (set `local.EmptyClip` (<= _weapondata_currentammoinclip 0))
  (return (and (`local.EmptyAmmo`) (`local.EmptyClip`))))

(fn `IsOwnerEquipWeapon`
  (returns (Result :type Boolean))
  (locals (OwnerWeaponClass :type "/Game/Weapon/Base/BaseWeapon_BP Class Reference"))
  (`/Engine/EditorBlueprintResources/StandardMacros.IsValid` (`self.OwnerPawn`)
    (:`Is Valid`
      (set `local.OwnerWeaponClass` null))
    (:`Is Not Valid`
      (return false))))

(fn `SpawnFireEffects`
  (bind _returnvalue (`GameplayStatics.SpawnEmitterAtLocation` null (`self.TraceStart`)))
  (`FXSystemComponent.SetVectorParameter` _returnvalue "None" (`KismetMathLibrary.SelectVector` (`self.TraceHitLocation`) (`self.TraceEnd`)))
  (`GameplayStatics.PlaySoundAtLocation` (`self.FireSound`) (`SceneComponent.K2_GetComponentLocation` (`self.Muzzle`)) (struct) 1.0 1.0 0.0 null null null)
  (return))

(fn `UserConstructionScript`)